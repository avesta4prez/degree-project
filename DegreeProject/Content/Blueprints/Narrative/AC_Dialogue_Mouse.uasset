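; Dialogue component for a Mouse character that asks for cheese and branches on whether it is offered, kept or unavailable.
; It overrides the parent Dialogue function, switching on DialogueTreeIndex and nesting AddDialogue calls that advance on Pass Through and branch by option index.
; Giving cheese moves the tree to index 1, which has no dialogue here.
; Refusals roll back or clear dialogue progress, then close the conversation.
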(event EventBeginPlay)

(event EventTick
  (params (DeltaSeconds :type Float%20%28single-precision%29)))

(fn Dialogue
  (|CallParentFunction)
  (switch int (Variables|Default|GetDialogueTreeIndex)
    (:0
      (bind (_state _optionindex) (CallFunction|AddDialogue "Mouse" "Hi, do you have any cheese?" (Utilities|Array|MakeArray "Yes" "No")))
      (switch Utilities|FlowControl|Switch|SwitchonEnum_DialogueState _state
        (:NewEnumerator0
          (switch int _optionindex
            (:0
              (bind (_state_2 _optionindex_2) (CallFunction|AddDialogue "Mouse" "Ahh, that's great news, can I have some?" (Utilities|Array|MakeArray "Give Cheese" "Keep Cheese")))
              (switch Utilities|FlowControl|Switch|SwitchonEnum_DialogueState _state_2
                (:NewEnumerator0
                  (switch int _optionindex_2
                    (:0
                      (bind _state_3 (CallFunction|AddDialogue "Mouse" "Thank you, thank you!! You're so kind" (Utilities|Array|MakeArray "Continue")))
                      (switch Utilities|FlowControl|Switch|SwitchonEnum_DialogueState _state_3
                        (:NewEnumerator0
                          (CallFunction|SetDialogueTreeIndex 1))))
                    (:1
                      (bind _state_4 (CallFunction|AddDialogue "Mouse" "You big meanie!" (Utilities|Array|MakeArray "Continue")))
                      (switch Utilities|FlowControl|Switch|SwitchonEnum_DialogueState _state_4
                        (:NewEnumerator0
                          (CallFunction|RemoveDialogueProgress 2)
                          (CallFunction|CloseConversation))))))))
            (:1
              (bind _state_5 (CallFunction|AddDialogue "Mouse" "Aww, that's a shame. I reall want some cheese" (Utilities|Array|MakeArray "Continue")))
              (switch Utilities|FlowControl|Switch|SwitchonEnum_DialogueState _state_5
                (:NewEnumerator0
                  (CallFunction|ClearDialogueProgress)
                  (CallFunction|CloseConversation))))))))))