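; Player build-mode component that previews, places and moves buildables loaded from a data table.
; A camera line trace, repeated on a short delay loop, positions a ghost mesh, snapping it to build boxes reported by the hit actor.
; Overlap and downward ground traces color the ghost green or red and set CanBuild.
; SpawnBuild spawns the selected actor, passing mesh and cost data via messages, or relocates the actor being moved.
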(event Custom|BuildDelay
  (bind _buildghost (Variables|Default|GetBuildGhost))
  ;[0.05098 0.05098 0.05098] Build Delay
  (if (Variables|Default|GetIsBuildModeOn)
    (Utilities|FlowControl|Delay 0.01)
    (CallFunction|BuildCycle)
    (else
      (Variables|Default|SetIsBuildModeOn false)
      (Variables|Default|SetCanBuild false)
      (Variables|Default|SetMovableActor 0)
      (Variables|Default|SetIsMoving? false)
      (Utilities|IsValid _buildghost
        (:Is%20Valid
          (Default|DestroyComponent (Variables|Default|GetPlayerRef) _buildghost))))))

(event Custom|StopBuildMode
  (bind _buildghost (Variables|Default|GetBuildGhost))
  ;[0.05098 0.05098 0.05098] Build Delay
  (Variables|Default|SetIsBuildModeOn false)
  (Variables|Default|SetCanBuild false)
  (Variables|Default|SetMovableActor 0)
  (Variables|Default|SetIsMoving? false)
  (Utilities|IsValid _buildghost
    (:Is%20Valid
      (Default|DestroyComponent (Variables|Default|GetPlayerRef) _buildghost))))

(event Custom|LaunchBuildMode
  ;[0.05098 0.05098 0.05098] Launch Build Mode
  (if (Variables|Default|GetIsBuildModeOn)
    (CallFunction|StopBuildMode)
    (else
      (Variables|Default|SetIsBuildModeOn true)
      (CallFunction|BuildCycle))))

(event EventBeginPlay
  ;[0.05098 0.05098 0.05098] Get Buildables DB
  (bind _asbp_third_person_character (Utilities|Casting|CastToBP_ThirdPersonCharacter (Components|GetOwner)))
  (Variables|Default|SetPlayerRef _asbp_third_person_character)
  (bind _outrownames (DataTable|GetDataTableRowNames "/Game/Blueprints/BuildSystem/BuildablesDB.BuildablesDB"))
  (for _array_element _outrownames
    (bind _returnvalue (Utilities|GetDataTableRow "/Game/Blueprints/BuildSystem/BuildablesDB.BuildablesDB" _array_element)
      (:then
        (Utilities|Array|Add (Variables|Default|GetBuildables) _returnvalue)))))

(fn SpawnBuildGhost
  (bind _returnvalue (Game|AddComponentbyClass (Variables|Default|GetPlayerRef) "/Script/Engine.StaticMeshComponent" false (Variables|Default|GetBuildTransform)))
  (bind _output_get (Variables|Default|SetBuildGhost _returnvalue))
  (Components|StaticMesh|SetStaticMesh _output_get (.mesh (Utilities|Array|Get(acopy) (Variables|Default|GetBuildables) (Variables|Default|GetBuildID))))
  (Collision|SetCollisionEnabled (Variables|Default|GetBuildGhost) "NoCollision"))

(fn GiveBuildColor
  (params (IsGreen :type Boolean))
  (bind _buildghost (Variables|Default|GetBuildGhost))
  (Variables|Default|SetCanBuild IsGreen)
  (for _index (range 0 (- (Rendering|Material|GetNumMaterials (Variables|Default|GetBuildGhost)) 1))
    (if IsGreen
      (Rendering|Material|SetMaterial _buildghost _index "/Game/Assets/GreenColor.GreenColor")
      (else
        (Rendering|Material|SetMaterial _buildghost _index "/Game/Assets/RedColor.RedColor"))))
  (Transformation|SetWorldTransform (Variables|Default|GetBuildGhost) (Variables|Default|GetBuildTransform) false false))

(fn BuildCycle
  (bind _camera (Variables|Default|GetCamera))
  (bind _buildghost (Variables|Default|GetBuildGhost))
  (bind _returnvalue (Transformation|GetWorldLocation _camera))
  (bind _returnvalue_2 (Math|Vector|GetForwardVector _camera))
  (bind (_outhit _returnvalue_3) (Collision|LineTraceByChannel (+ _returnvalue (* _returnvalue_2 350)) (+ _returnvalue (* _returnvalue_2 1000)) (.tracechannel (Utilities|Array|Get(acopy) (Variables|Default|GetBuildables) (Variables|Default|GetBuildID))) false 0 "None"))
  (if _returnvalue_3
    (Variables|Default|SetBuildTransform (Math|Transform|MakeTransform (.ImpactPoint (Collision|BreakHitResult _outhit)) (.rotation (Variables|Default|GetBuildTransform)) (.scale (Variables|Default|GetBuildTransform))))
    (Variables|Default|SetHit%20Actor (.HitActor (Collision|BreakHitResult _outhit)))
    (Variables|Default|SetHit%20Component (.HitComponent (Collision|BreakHitResult _outhit)))
    (Utilities|IsValid _buildghost
      (:Is%20Valid
        (bind (_found _transform) (CallFunction|DetectBuildBoxes))
        (if _found
          (Variables|Default|SetBuildTransform _transform))
        (bind _hit (CallFunction|CheckforOverlap))
        (bind _didhit (CallFunction|IsBuildFloating))
        (CallFunction|GiveBuildColor (and _didhit (not _hit)))
        (CallFunction|BuildDelay))
      (:Is%20Not%20Valid
        (CallFunction|SpawnBuildGhost :!label _label)
        (CallFunction|BuildDelay :!label _label_2)))
    (else
      (Variables|Default|SetBuildTransform (Math|Transform|MakeTransform (.TraceEnd (Collision|BreakHitResult _outhit)) (.rotation (Variables|Default|GetBuildTransform)) (.scale (Variables|Default|GetBuildTransform))))
      (Utilities|IsValid _buildghost
        (:Is%20Valid
          (CallFunction|GiveBuildColor false)
          (goto _label_2))
        (:Is%20Not%20Valid
          (goto _label))))))

(fn ChangeMesh
  (Components|StaticMesh|SetStaticMesh (Variables|Default|GetBuildGhost) (.mesh (Utilities|Array|Get(acopy) (Variables|Default|GetBuildables) (Variables|Default|GetBuildID)))))

(fn SpawnBuild
  (bind _buildables (Variables|Default|GetBuildables))
  (bind _buildid (Variables|Default|GetBuildID))
  (bind _output (Utilities|Array|Get(acopy) _buildables _buildid))
  (if (Variables|Default|GetIsMoving?)
    (Transformation|SetActorTransform (Variables|Default|GetMovableActor) (Variables|Default|GetBuildTransform))
    (CallFunction|StopBuildMode)
    (else
      (bind _returnvalue (Game|SpawnActorfromClass (.actor _output) (Variables|Default|GetBuildTransform) "Undefined" "MultiplyWithRoot" 0 0))
      (Class|BuildInterface|SetMesh(Message) _returnvalue (.mesh _output))
      (Class|BuildInterface|SetBuildCost(Message) _returnvalue (Utilities|Array|Get(acopy) (Variables|Default|GetBuildables) (Variables|Default|GetBuildID)) (Variables|Default|GetBuildID)))))

(fn DetectBuildBoxes
  (bind _boxes (Class|BuildInterface|ReturnBoxes(Message) (Variables|Default|GetHit%20Actor)))
  (bind _array_element (Utilities|Array|ForEachLoopwithBreak _boxes :!label _label)
    (:LoopBody
      (if (== _array_element (Variables|Default|GetHit%20Component))
        (LocalVariables|SetLocalFound true)
        (goto _label Break)))
    (:Completed
      (return (LocalVariables|GetLocalFound) (Transformation|GetWorldTransform (Variables|Default|GetHit%20Component))))))

(fn CheckforOverlap
  (bind _buildghost (Variables|Default|GetBuildGhost))
  (bind (_origin _boxextent) (Collision|GetComponentBounds _buildghost))
  (bind _returnvalue (Collision|BoxTraceByChannel _origin _origin (/ _boxextent 1.2) "0, 0, 0" "TraceTypeQuery1" false 0 "None"))
  (return _returnvalue))

(fn IsBuildFloating
  (bind _buildtransform (Variables|Default|GetBuildTransform))
  (bind _returnvalue (Collision|LineTraceByChannel (.location _buildtransform) (- (.location _buildtransform) "0.000000,0.000000,500.000000") "TraceTypeQuery1" false 0 "None"))
  (return _returnvalue))

(fn MoveBuildable
  (bind _buildid (Class|BuildInterface|ReturnBuildID(Message) (Variables|Default|GetMovableActor)))
  (Variables|Default|SetBuildID _buildid)
  (CallFunction|LaunchBuildMode))