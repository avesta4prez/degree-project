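; Inventory component in the Shopkeeper folder that tracks item quantities in a map keyed by item ID.
; AddToInventory stacks the given quantity onto an existing entry or creates a new one.
; RemoveFromInventory takes one unit off an existing item and deletes its entry when the count reaches zero or below.
; The event graph holds no active logic, so all changes come through these two functions.
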(event EventBeginPlay)

(event EventTick
  (params (DeltaSeconds :type Float%20%28single-precision%29)))

(fn AddtoInventory
  (params (ItemID :type Integer) (Quantity :type Integer))
  (bind _inventorymap (Variables|Default|GetInventoryMap))
  (bind (_value _returnvalue) (Utilities|Map|Find _inventorymap ItemID))
  (if _returnvalue
    (Utilities|Map|Add (Variables|Default|GetInventoryMap) ItemID (+ Quantity _value))
    (else
      (Utilities|Map|Add (Variables|Default|GetInventoryMap) ItemID Quantity)))
  (return))

(fn RemovefromInventory
  (params (ItemID :type Integer))
  (bind _inventorymap (Variables|Default|GetInventoryMap))
  (bind _inventorymap_2 (Variables|Default|GetInventoryMap))
  (bind (_value _returnvalue) (Utilities|Map|Find _inventorymap ItemID))
  (bind _returnvalue_2 (- _value 1))
  (if _returnvalue
    (if (<= _returnvalue_2 0)
      (Utilities|Map|Remove _inventorymap_2 ItemID)
      (else
        (Utilities|Map|Add _inventorymap_2 ItemID _returnvalue_2)))))