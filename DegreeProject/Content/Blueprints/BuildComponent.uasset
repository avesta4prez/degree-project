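; Actor component for BP_ThirdPersonCharacter that runs a toggleable build mode previewing a Foundation mesh.
; While active, BuildCycle and BuildDelay re-trigger each other through a short delay, line-tracing ahead of the camera.
; A collisionless ghost mesh follows the impact point or trace end, turning green on a hit or red otherwise and setting CanBuild.
; Stopping clears the flags and destroys the ghost; no placement happens here.
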(event Custom|BuildDelay
  (bind _buildghost (Variables|Default|GetBuildGhost))
  (if (Variables|Default|GetIsBuildModeOn)
    (Utilities|FlowControl|Delay 0.01)
    (CallFunction|BuildCycle)
    (else
      (Variables|Default|SetIsBuildModeOn false)
      (Variables|Default|SetCanBuild false)
      (Utilities|IsValid _buildghost
        (:Is%20Valid
          (Default|DestroyComponent (Variables|Default|GetPlayerRef) _buildghost))))))

(event Custom|StopBuildMode
  (bind _buildghost (Variables|Default|GetBuildGhost))
  (Variables|Default|SetIsBuildModeOn false)
  (Variables|Default|SetCanBuild false)
  (Utilities|IsValid _buildghost
    (:Is%20Valid
      (Default|DestroyComponent (Variables|Default|GetPlayerRef) _buildghost))))

(event Custom|LaunchBuildMode
  (if (Variables|Default|GetIsBuildModeOn)
    (CallFunction|StopBuildMode)
    (else
      (Variables|Default|SetIsBuildModeOn true)
      (CallFunction|BuildCycle))))

(event EventBeginPlay
  (bind _asbp_third_person_character (Utilities|Casting|CastToBP_ThirdPersonCharacter (Components|GetOwner)))
  (Variables|Default|SetPlayerRef _asbp_third_person_character))

(fn SpawnBuildGhost
  (bind _returnvalue (Game|AddComponentbyClass (Variables|Default|GetPlayerRef) "/Script/Engine.StaticMeshComponent" false (Variables|Default|GetBuildTransform)))
  (bind _output_get (Variables|Default|SetBuildGhost _returnvalue))
  (Components|StaticMesh|SetStaticMesh _output_get "/Game/Assets/Build/foundation.foundation")
  (Collision|SetCollisionEnabled (Variables|Default|GetBuildGhost) "NoCollision"))

(fn GiveBuildColor
  (params (IsGreen :type Boolean))
  (bind _buildghost (Variables|Default|GetBuildGhost))
  (Variables|Default|SetCanBuild IsGreen)
  (for _index (range 0 (- (Rendering|Material|GetNumMaterials (Variables|Default|GetBuildGhost)) 1))
    (if IsGreen
      (Rendering|Material|SetMaterial _buildghost _index "/Game/Assets/GreenColor.GreenColor")
      (else
        (Rendering|Material|SetMaterial _buildghost _index "/Game/Assets/RedColor.RedColor"))))
  (Transformation|SetWorldTransform (Variables|Default|GetBuildGhost) (Variables|Default|GetBuildTransform) false false))

(fn BuildCycle
  (bind _camera (Variables|Default|GetCamera))
  (bind _buildghost (Variables|Default|GetBuildGhost))
  (bind _returnvalue (Transformation|GetWorldLocation _camera))
  (bind _returnvalue_2 (Math|Vector|GetForwardVector _camera))
  (bind (_outhit _returnvalue_3) (Collision|LineTraceByChannel (+ _returnvalue (* _returnvalue_2 350)) (+ _returnvalue (* _returnvalue_2 1000)) "TraceTypeQuery1" false 0 "None"))
  (if _returnvalue_3
    (Variables|Default|SetBuildTransform (Math|Transform|MakeTransform (.ImpactPoint (Collision|BreakHitResult _outhit)) (.rotation (Variables|Default|GetBuildTransform)) (.scale (Variables|Default|GetBuildTransform))))
    (Utilities|IsValid _buildghost
      (:Is%20Valid
        (CallFunction|GiveBuildColor true))
      (:Is%20Not%20Valid
        (CallFunction|SpawnBuildGhost :!label _label)))
    (else
      (Variables|Default|SetBuildTransform (Math|Transform|MakeTransform (.TraceEnd (Collision|BreakHitResult _outhit)) (.rotation (Variables|Default|GetBuildTransform)) (.scale (Variables|Default|GetBuildTransform))))
      (Utilities|IsValid _buildghost
        (:Is%20Valid
          (CallFunction|GiveBuildColor false))
        (:Is%20Not%20Valid
          (goto _label)))))
  (CallFunction|BuildDelay))